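; Player controller for the multiplayer JUMP game, handling respawning, level tracking, high scores, chat and the in-game menu.
; Resolves the Steam or PlayerState name, retrying by timer, before reporting loaded so the GameMode announces the join and checks scores.
; A LevelTracker component, replaced on level entry, supplies the respawn transform.
; Server events relay respawns and chat to the GameMode and submit locally saved best results to each LevelManager.
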(event Custom|EnterLevel
  (params (LevelInfo :type Level%20Info%20Structure) (LevelManager :type Level%20Manager%20Object%20Reference))
  (Utilities|IsValid (Variables|Default|GetCurrentLevelTracker)
    (:Is%20Valid
      (Components|DestroyComponent (Variables|Default|GetCurrentLevelTracker)))
    (:Is%20Not%20Valid
      _))
  (bind _returnvalue (AddComponent|AddLevelTracker self))
  (bind _output_get (Variables|Default|SetCurrentLevelTracker _returnvalue))
  (Default|Initialize _output_get LevelInfo LevelManager))

(event Custom|Respawn
  (bind _currentleveltracker (Variables|Default|GetCurrentLevelTracker))
  (Utilities|IsValid _currentleveltracker
    (:Is%20Valid
      (CallFunction|ServerRespawnLevel (.RespawnTransform (Utilities|Struct|BreakLevelInfo (Variables|/Game/Blueprints/LevelTracker.LevelTracker_C|GetLevelInfo _currentleveltracker))))
      (Default|Reset _currentleveltracker))))

(event Custom|ShowChatBox
  (bind _self self)
  (Utilities|IsValid (Variables|Default|GetChatbox)
    (:Is%20Not%20Valid
      (bind _returnvalue (UserInterface|CreateWidget "/Game/Blueprints/UI/ChatBox.ChatBox_C" _self _self))
      (bind _output_get (Variables|Default|SetChatbox _returnvalue))
      (UserInterface|Viewport|AddtoViewport _output_get 0))))

(event Custom|RPC_SendMessage
  (params (MessageToSend :type Text) (PlayerName :type String))
  (bind _asjump_game_mode (Utilities|Casting|CastToJUMP_GameMode (Game|GetGameMode)))
  (Default|NewMessage _asjump_game_mode PlayerName MessageToSend))

(event Custom|OnSendMessage
  (params (Message :type Text))
  (CallFunction|RPCSendMessage Message (Variables|Default|GetNetName))
  (Input|SetInputModeGameOnly self))

(event Custom|Server_RequestHighScoreCheck
  (bind _asjump_game_mode (Utilities|Casting|CastToJUMP_GameMode (Game|GetGameMode)))
  (Default|Alert _asjump_game_mode (Utilities|Text|FormatText "{Name} has joined the server." (Utilities|Text|ToText(String) (Variables|Default|GetNetName))) "(R=0.000000,G=0.041267,B=0.895833,A=1.000000)")
  (Default|CheckPlayerHighScores _asjump_game_mode self))

(event Custom|LocalCheckHighscores
  (params (lvel%20managers :type Array%20of%20Level%20Manager%20Object%20References))
  (Default|LoadPlayer (.AsJump%20Game%20Instance (Utilities|Casting|CastToJumpGameInstance (Game|GetGameInstance))))
  (for _array_element lvel%20managers
    (CallFunction|UpdateHighscoreText (Variables|/Game/Blueprints/Scene/LevelManager.LevelManager_C|GetHighScoreText _array_element))
    (if (.Completed? (Utilities|Struct|BreakPlayerLevelInfo (Utilities|Array|Get(acopy) (Variables|/Game/Blueprints/JumpGameInstance.JumpGameInstance_C|GetCurrentPlayerScores (.AsJump%20Game%20Instance (Utilities|Casting|CastToJumpGameInstance (Game|GetGameInstance)))) (.levelindex (Variables|/Game/Blueprints/Scene/LevelManager.LevelManager_C|GetLevelInfo _array_element)))))
      (CallFunction|ServerCompareHighScore (.BestResult (Utilities|Struct|BreakPlayerLevelInfo (Utilities|Array|Get(acopy) (Variables|/Game/Blueprints/JumpGameInstance.JumpGameInstance_C|GetCurrentPlayerScores (.AsJump%20Game%20Instance (Utilities|Casting|CastToJumpGameInstance (Game|GetGameInstance)))) (.levelindex (Variables|/Game/Blueprints/Scene/LevelManager.LevelManager_C|GetLevelInfo _array_element))))) (Utilities|Text|ToText(String) (Variables|Default|GetNetName)) _array_element))))

(event Custom|Load
  (CallFunction|LocalHasCompletedTutorial?)
  (if (Variables|Default|GetIsNameSet?)
    (CallFunction|LoadComplete)
    (else
      (EventDispatchers|BindEventtoOnNameInitialized (delegate Custom|LoadComplete))
      (CallFunction|SetNetName))))

(event Custom|ReceiveAlert
  (params (Message :type Text) (Color :type Linear%20Color%20Structure))
  (CallFunction|ShowChatBox)
  (Default|ReceiveAlert (Variables|Default|GetChatbox) Message Color))

(event Custom|Server_SetLoaded
  (params (Name :type String))
  (Variables|Default|SetIsLoaded? true)
  (Variables|Default|SetNetName Name)
  (CallFunction|ServerRequestHighScoreCheck))

(event Custom|Server_SetTutorial
  (params (value :type Boolean))
  (Variables|Default|SetCompletedTutorial? value))

(event Custom|LoadComplete
  (Variables|Default|SetIsLoaded? true)
  (CallFunction|ServerSetLoaded (Variables|Default|GetNetName)))

(event Custom|ExitLevel
  (bind _currentleveltracker (Variables|Default|GetCurrentLevelTracker))
  (Utilities|IsValid _currentleveltracker
    (:Is%20Valid
      (Default|RemoveLevelUI _currentleveltracker)
      (Default|UpdateStats _currentleveltracker)
      (Components|DestroyComponent _currentleveltracker))))

(event Custom|UpdateHighscoreText
  (params (Target :type High%20Score%20Text%20Object%20Reference))
  (Default|GetServerHighScore Target))

(event Custom|ReceiveMessage
  (params (PlayerName :type String) (Message :type Text))
  (CallFunction|ShowChatBox)
  (Default|ReceiveMessage (Variables|Default|GetChatbox) PlayerName Message))

(event Custom|Server_Respawn_Level
  (params (RespawnTransform :type Transform))
  (bind _asjump_game_mode (Utilities|Casting|CastToJUMP_GameMode (Game|GetGameMode)))
  (Default|RespanPlayer _asjump_game_mode self RespawnTransform))

(event Custom|Server_Respawn
  (bind _asjump_game_mode (Utilities|Casting|CastToJUMP_GameMode (Game|GetGameMode)))
  (Default|SpawnPlayer _asjump_game_mode self))

(event Custom|SetNetName
  (bind _playerstate (Variables|GetPlayerState))
  (if (Class|VictoryBPFunctionLibrary|StringIsEmpty (Variables|Default|GetNetName))
    (Utilities|IsValid _playerstate
      (:Is%20Valid
        (bind _returnvalue (Class|AdvancedSteamFriendsLibrary|GetSteamPersonaName (Class|AdvancedSessionsLibrary|GetUniqueNetIDfromPlayerState _playerstate)))
        (bind _output_get (Variables|Default|SetNetName _returnvalue))
        (if (Class|VictoryBPFunctionLibrary|StringIsEmpty _output_get)
          (bind _output_get_2 (Variables|Default|SetNetName (PlayerState|GetPlayerName _playerstate)))
          (if (Class|VictoryBPFunctionLibrary|StringIsEmpty _output_get_2)
            (Utilities|Time|SetTimerbyEvent (delegate Custom|SetNetName) 1.0)
            (else
              (Variables|Default|SetIsNameSet? true :!label _label)
              (Default|CallOnNameInitialized)))
          (else
            (goto _label))))
      (:Is%20Not%20Valid
        (Utilities|Time|SetTimerbyEvent (delegate Custom|SetNetName) 1.0)))
    (else
      (Variables|Default|SetIsNameSet? true))))

(event Custom|Server_CompareHighScore
  (params (Result :type Level%20Result%20Structure) (PlayerName :type Text) (Level%20manager :type Level%20Manager%20Object%20Reference))
  (Default|CompareResults Level%20manager Result PlayerName))

(event Custom|Local_HasCompletedTutorial?
  (bind _asjump_game_instance (Utilities|Casting|CastToJumpGameInstance (Game|GetGameInstance)))
  (bind _output_get (Variables|Default|SetCompletedTutorial? (Variables|/Game/Blueprints/JumpGameInstance.JumpGameInstance_C|GetHasCompletedTutorial? _asjump_game_instance)))
  (CallFunction|ServerSetTutorial _output_get))

(event EventBeginPlay
  (Class|WidgetBlueprintLibrary|SetFocustoGameViewport)
  (Input|SetInputModeGameOnly self)
  (CallFunction|SetNetName))

(event EventTick
  (params (DeltaSeconds :type Float%20%28single-precision%29)))

(event Input|ActionEvents|InputActionOpenMenu
  (params (Key :type Key%20Structure :default "None"))
  (:Pressed
    (bind _asjump_game_instance (Utilities|Casting|CastToJumpGameInstance (Game|GetGameInstance)))
    (Default|ShowIngameMenu _asjump_game_instance)))

(event Input|ActionEvents|InputActionForceRespawn
  (params (Key :type Key%20Structure :default "None"))
  (:Pressed
    (Utilities|IsValid (Variables|Default|GetCurrentLevelTracker)
      (:Is%20Valid
        (bind _output_get (Variables|Default|SetcurrentRotation (Pawn|GetControlRotation :!class /Script/Engine.Controller)))
        (CallFunction|Respawn)
        (Pawn|SetControlRotation _output_get))
      (:Is%20Not%20Valid
        (CallFunction|ServerRespawn)))))

(event Input|ActionEvents|InputActionSendMessage
  (params (Key :type Key%20Structure :default "None"))
  (:Pressed
    (CallFunction|ShowChatBox)
    (Default|OnStartTyping (Variables|Default|GetChatbox))))

(fn ConstructionScript)

(fn GetPlayerRef
  (bind _returnvalue (Pawn|GetControlledPawn))
  (Utilities|IsValid _returnvalue
    (:Is%20Valid
      (bind _asjump_player (Utilities|Casting|CastToJUMP_Player _returnvalue)
        (:then
          (return _asjump_player true))
        (:CastFailed
          _)))
    (:Is%20Not%20Valid
      _))
  (return 0 false))