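; Configurable level block that forms a hollow grid of meshes which can rotate or travel along a spline, or a single physics-simulated mesh.
; The construction script builds the shell around a pivot, using instanced meshes when static and separate components when moving or rotating.
; Tick accumulates rotation, while a timeline drives spline movement with bounce, loop, play-once or teleport-reset modes.
; The authority fires the movement-start dispatcher, and teleport resets briefly make blocks unwalkable.
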(event Custom|StartMovement
  (bind _targetpath (Variables|Default|GetTargetPath))
  ;[1 1 1] Movement Handler
  (if (not (Variables|Movement|GethasStarted?))
    (Variables|Movement|SethasStarted? true)
    (bind (_direction _alpha) (Timeline|BlockMover Play)
      (:Update
        (Utilities|IsValid (Variables|Default|GetTargetPath)
          (:Is%20Valid
            (Variables|Movement|SetMovementAlpha _alpha)
            (Variables|Movement|SetcurrentDirection _direction)
            (if (Variables|Movement|GetInheritSplineRotation?)
              (Transformation|SetWorldLocationAndRotation (Variables|Object|GetblockRoot) (Spline|GetLocationatDistanceAlongSpline _targetpath (Math|Float|Lerp 0.0 (Variables|Movement|GetSplineLength) (Variables|Movement|GetMovementAlpha)) "World") (Math|Rotator|CombineRotators (Variables|Movement|GetCurrentRotation) (Spline|GetRotationatDistanceAlongSpline _targetpath (Math|Float|Lerp 0.0 (Variables|Movement|GetSplineLength) (Variables|Movement|GetMovementAlpha)) "World")) false false)
              (else
                (Transformation|SetWorldLocation (Variables|Object|GetblockRoot) (Spline|GetLocationatDistanceAlongSpline _targetpath (Math|Float|Lerp 0.0 (Variables|Movement|GetSplineLength) (Variables|Movement|GetMovementAlpha)) "World") false false)
                (Transformation|SetWorldRotation (Variables|Object|GetblockRoot) (Variables|Movement|GetCurrentRotation) false false))))))
      (:Finished
        (CallFunction|OnMovementFinished)))))

(event Custom|InitMover
  (bind _targetpath (Variables|Default|GetTargetPath))
  (bind _splinelength (Variables|Movement|GetSplineLength))
  (bind _movementalpha (Variables|Movement|GetMovementAlpha))
  (bind _returnvalue (Math|Float|Lerp 0.0 _splinelength _movementalpha))
  (bind _returnvalue_2 (Spline|GetLocationatDistanceAlongSpline _targetpath _returnvalue "World"))
  ;[1 1 1] Movement Handler
  (if (Variables|Movement|GetInheritSplineRotation?)
    (Transformation|SetWorldLocationAndRotation (Variables|Object|GetblockRoot) _returnvalue_2 (Math|Rotator|CombineRotators (Variables|Movement|GetCurrentRotation) (Spline|GetRotationatDistanceAlongSpline _targetpath _returnvalue "World")) false false)
    (else
      (Transformation|SetWorldLocation (Variables|Object|GetblockRoot) _returnvalue_2 false false)
      (Transformation|SetWorldRotation (Variables|Object|GetblockRoot) (Variables|Movement|GetCurrentRotation) false false))))

(event Custom|StopMovement
  (bind _targetpath (Variables|Default|GetTargetPath))
  ;[1 1 1] Movement Handler
  (Variables|Movement|SethasStarted? false)
  (bind (_direction _alpha) (Timeline|BlockMover Stop)
    (:Update
      (Utilities|IsValid (Variables|Default|GetTargetPath)
        (:Is%20Valid
          (Variables|Movement|SetMovementAlpha _alpha)
          (Variables|Movement|SetcurrentDirection _direction)
          (if (Variables|Movement|GetInheritSplineRotation?)
            (Transformation|SetWorldLocationAndRotation (Variables|Object|GetblockRoot) (Spline|GetLocationatDistanceAlongSpline _targetpath (Math|Float|Lerp 0.0 (Variables|Movement|GetSplineLength) (Variables|Movement|GetMovementAlpha)) "World") (Math|Rotator|CombineRotators (Variables|Movement|GetCurrentRotation) (Spline|GetRotationatDistanceAlongSpline _targetpath (Math|Float|Lerp 0.0 (Variables|Movement|GetSplineLength) (Variables|Movement|GetMovementAlpha)) "World")) false false)
            (else
              (Transformation|SetWorldLocation (Variables|Object|GetblockRoot) (Spline|GetLocationatDistanceAlongSpline _targetpath (Math|Float|Lerp 0.0 (Variables|Movement|GetSplineLength) (Variables|Movement|GetMovementAlpha)) "World") false false)
              (Transformation|SetWorldRotation (Variables|Object|GetblockRoot) (Variables|Movement|GetCurrentRotation) false false))))))
    (:Finished
      (CallFunction|OnMovementFinished))))

(event Custom|StartMovementReverse
  (bind _targetpath (Variables|Default|GetTargetPath))
  ;[1 1 1] Movement Handler
  (bind (_direction _alpha) (Timeline|BlockMover ReverseFromEnd)
    (:Update
      (Utilities|IsValid (Variables|Default|GetTargetPath)
        (:Is%20Valid
          (Variables|Movement|SetMovementAlpha _alpha)
          (Variables|Movement|SetcurrentDirection _direction)
          (if (Variables|Movement|GetInheritSplineRotation?)
            (Transformation|SetWorldLocationAndRotation (Variables|Object|GetblockRoot) (Spline|GetLocationatDistanceAlongSpline _targetpath (Math|Float|Lerp 0.0 (Variables|Movement|GetSplineLength) (Variables|Movement|GetMovementAlpha)) "World") (Math|Rotator|CombineRotators (Variables|Movement|GetCurrentRotation) (Spline|GetRotationatDistanceAlongSpline _targetpath (Math|Float|Lerp 0.0 (Variables|Movement|GetSplineLength) (Variables|Movement|GetMovementAlpha)) "World")) false false)
            (else
              (Transformation|SetWorldLocation (Variables|Object|GetblockRoot) (Spline|GetLocationatDistanceAlongSpline _targetpath (Math|Float|Lerp 0.0 (Variables|Movement|GetSplineLength) (Variables|Movement|GetMovementAlpha)) "World") false false)
              (Transformation|SetWorldRotation (Variables|Object|GetblockRoot) (Variables|Movement|GetCurrentRotation) false false))))))
    (:Finished
      (CallFunction|OnMovementFinished))))

(event Custom|StartMovementForward
  (bind _targetpath (Variables|Default|GetTargetPath))
  ;[1 1 1] Movement Handler
  (bind (_direction _alpha) (Timeline|BlockMover PlayFromStart)
    (:Update
      (Utilities|IsValid (Variables|Default|GetTargetPath)
        (:Is%20Valid
          (Variables|Movement|SetMovementAlpha _alpha)
          (Variables|Movement|SetcurrentDirection _direction)
          (if (Variables|Movement|GetInheritSplineRotation?)
            (Transformation|SetWorldLocationAndRotation (Variables|Object|GetblockRoot) (Spline|GetLocationatDistanceAlongSpline _targetpath (Math|Float|Lerp 0.0 (Variables|Movement|GetSplineLength) (Variables|Movement|GetMovementAlpha)) "World") (Math|Rotator|CombineRotators (Variables|Movement|GetCurrentRotation) (Spline|GetRotationatDistanceAlongSpline _targetpath (Math|Float|Lerp 0.0 (Variables|Movement|GetSplineLength) (Variables|Movement|GetMovementAlpha)) "World")) false false)
            (else
              (Transformation|SetWorldLocation (Variables|Object|GetblockRoot) (Spline|GetLocationatDistanceAlongSpline _targetpath (Math|Float|Lerp 0.0 (Variables|Movement|GetSplineLength) (Variables|Movement|GetMovementAlpha)) "World") false false)
              (Transformation|SetWorldRotation (Variables|Object|GetblockRoot) (Variables|Movement|GetCurrentRotation) false false))))))
    (:Finished
      (CallFunction|OnMovementFinished))))

(event Custom|DestroyAndReset
  (bind _targetpath (Variables|Default|GetTargetPath))
  ;[1 1 1] Destroy and Reset
  (for _array_element (Variables|Object|GetBlocks)
    (Class|PrimitiveComponent|SetWalkableSlopeOverride _array_element (Utilities|Struct|MakeWalkableSlopeOverride "WalkableSlope_Unwalkable" 0.0)))
  (Utilities|FlowControl|Delay 0.001)
  (Variables|Movement|SetMovementAlpha 0.0)
  (Transformation|SetWorldLocationAndRotation (Variables|Transformation|GetRootComponent) (Spline|GetLocationatDistanceAlongSpline _targetpath 0.0 "World") (Spline|GetRotationatDistanceAlongSpline _targetpath 0.0 "World") false true)
  (for _array_element_2 (Variables|Object|GetBlocks)
    (Class|PrimitiveComponent|SetWalkableSlopeOverride _array_element_2))
  (Networking|SwitchHasAuthority
    (:Authority
      (Default|CallOnStartMovement))
    (:Remote
      _))
  (CallFunction|StartMovementForward))

(event Custom|DoRotation
  (params (dt :type Float%20%28single-precision%29))
  ;[1 1 1] Rotation Handler
  (if (Variables|Movement|GetIsRotating?)
    (bind _rotation (CallFunction|GetFrameRotation dt))
    (Variables|Movement|SetCurrentRotation (Math|Rotator|CombineRotators _rotation (Variables|Movement|GetCurrentRotation)))
    (if (not (Variables|Movement|GetIsMoving?))
      (Transformation|SetWorldRotation (Variables|Object|GetblockRoot) (Variables|Movement|GetCurrentRotation) false false))))

(event Custom|OnMovementFinished
  ;[1 1 1] Movement Finished handler
  (switch Utilities|FlowControl|Switch|SwitchonMovementType (Variables|Movement|GetMovementType)
    (:NewEnumerator2
      (switch Utilities|FlowControl|Switch|SwitchonETimelineDirection (Variables|Movement|GetcurrentDirection)
        (:Forward
          (CallFunction|StartMovementReverse))
        (:Backward
          (Networking|SwitchHasAuthority :!label _label
            (:Authority
              (Default|CallOnStartMovement))
            (:Remote
              _))
          (CallFunction|StartMovementForward))))
    (:NewEnumerator0
      (goto _label))
    (:NewEnumerator3
      (CallFunction|DestroyandReset))
    (:NewEnumerator1
      (CallFunction|StopMovement))))

(event EventBeginPlay
  ;[1 1 1] Begin Play
  (EventDispatchers|BindEventtoOnStartMovement (delegate Custom|StartMovement))
  (Networking|SwitchHasAuthority
    (:Authority
      (if (Variables|Movement|GetIsMoving?)
        (if (Variables|Movement|GetAutoPlay?)
          (Default|CallOnStartMovement))))))

(event Collision|EventActorBeginOverlap
  (params (OtherActor :type Actor%20Object%20Reference)))

(event EventTick
  (params (DeltaSeconds :type Float%20%28single-precision%29))
  ;[1 1 1] Tick
  (CallFunction|DoRotation DeltaSeconds))

(fn ConstructionScript
  (bind _rotationduration (Variables|Movement|GetRotationDuration))
  (bind _rootblock (Variables|Default|GetrootBlock))
  (bind _rootblock_2 (Variables|Default|GetrootBlock))
  (bind _staticmesh (Variables|Object|GetStaticMesh))
  (bind _rootblock_3 (Variables|Default|GetrootBlock))
  (bind _returnvalue (StaticMesh|GetBounds _staticmesh))
  (if (Variables|Object|GetEnablePhysics?)
    (Components|StaticMesh|SetStaticMesh _rootblock_3 (Variables|Object|GetStaticMesh))
    (Rendering|Material|SetMaterial _rootblock_3 0 (Variables|Object|GetMaterial))
    (Physics|SetSimulatePhysics _rootblock_2 true)
    (Physics|SetEnableGravity _rootblock_2 true)
    (if (Variables|Object|GetIsWalkable?)
      (Class|PrimitiveComponent|SetWalkableSlopeOverride _rootblock)
      (else
        (Class|PrimitiveComponent|SetWalkableSlopeOverride _rootblock (Utilities|Struct|MakeWalkableSlopeOverride "WalkableSlope_Unwalkable" 0.0))))
    (else
      (Components|DestroyComponent (Variables|Default|GetrootBlock))
      ;[1 1 1] Set Mesh Extents
      (Variables|Dimensions|SetmeshW (* 2 (.x (.boxextent _returnvalue))))
      (Variables|Dimensions|SetmeshL (* 2 (.y (.boxextent _returnvalue))))
      (Variables|Dimensions|SetmeshH (* 2 (.z (.boxextent _returnvalue))))
      ;[1 1 1] Check is rotating
      (Variables|Movement|SetIsRotating? (Math|Boolean|ORBoolean (> (Math|Float|Absolute(Float) (.roll _rotationduration)) 0.0) (> (Math|Float|Absolute(Float) (.pitch _rotationduration)) 0.0) (> (Math|Float|Absolute(Float) (.yaw _rotationduration)) 0.0)))
      (Utilities|FlowControl|Sequence
        (:then_0
          ;[1 1 1] Check Mesh Type
          (if (Math|Boolean|ORBoolean (Variables|Movement|GetIsMoving?) (Variables|Movement|GetIsRotating?) (Variables|Object|GetEnablePhysics?))
            ;[1 1 1] set root block
            (Variables|Object|SetblockRoot (Variables|Transformation|GetRootComponent))
            (else
              ;[1 1 1] Create instanced mesh component, attach to pivot
              (bind _returnvalue_2 (AddComponent|AddInstancedStaticMeshComponent true))
              (bind _output_get (Variables|Object|SetInstancedMeshComponent _returnvalue_2))
              (Rendering|SetCastShadow _output_get false)
              (Transformation|AttachComponentToComponent _output_get (Variables|Transformation|GetRootComponent) "None" "KeepRelative" "KeepRelative" "KeepRelative" true)
              ;[1 1 1] Set Mesh
              (Components|StaticMesh|SetStaticMesh (Variables|Object|GetInstancedMeshComponent) (Variables|Object|GetStaticMesh))
              ;[1 1 1] Set Target Scene Comp
              (Variables|Object|SetblockRoot (Variables|Object|GetInstancedMeshComponent))))
          ;[1 1 1] Get pivot offset from mesh edge
          (Variables|Pivot|SetrootOffset (Math|Vector|MakeVector (/ (Variables|Dimensions|GetmeshW) 2.0) (/ (Variables|Dimensions|GetmeshL) 2.0) (/ (Variables|Dimensions|GetmeshH) 2.0)))
          ;[1 1 1] Get pivot point
          (Variables|Pivot|SetpivotPoint (+ (Math|Vector|MakeVector (* -1 (* (Variables|Dimensions|GetWidth) (* (Variables|Pivot|GetPivotW) (Variables|Dimensions|GetmeshW)))) (* -1 (* (Variables|Dimensions|GetLength) (* (Variables|Pivot|GetPivotL) (Variables|Dimensions|GetmeshL)))) (* -1 (* (Variables|Dimensions|GetHeight) (* (Variables|Pivot|GetPivotH) (Variables|Dimensions|GetmeshH))))) (Variables|Pivot|GetrootOffset))))
        (:then_1
          ;[1 1 1] Loop through all blocks
          (for _index (range 0 (- (Variables|Dimensions|GetWidth) 1))
            (Variables|Dimensions|SetcurrentWidth _index)
            (Variables|Dimensions|SetcurrentLength 0)
            (for _index_2 (range 0 (- (Variables|Dimensions|GetLength) 1))
              (Variables|Dimensions|SetcurrentLength _index_2)
              (Variables|Dimensions|SetcurrentHeight 0)
              (for _index_3 (range 0 (- (Variables|Dimensions|GetHeight) 1))
                (Variables|Dimensions|SetcurrentHeight _index_3)
                (if (Math|Boolean|ORBoolean (or (== (Variables|Dimensions|GetcurrentWidth) 0) (== (Variables|Dimensions|GetcurrentWidth) (- (Variables|Dimensions|GetWidth) 1))) (or (== (Variables|Dimensions|GetcurrentLength) 0) (== (Variables|Dimensions|GetcurrentLength) (- (Variables|Dimensions|GetLength) 1))) (or (== (Variables|Dimensions|GetcurrentHeight) 0) (== (Variables|Dimensions|GetcurrentHeight) (- (Variables|Dimensions|GetHeight) 1))))
                  ;[1 1 1] Check Mesh Type
                  (if (Math|Boolean|ORBoolean (Variables|Movement|GetIsMoving?) (Variables|Movement|GetIsRotating?) (Variables|Object|GetEnablePhysics?))
                    ;[1 1 1] Add static block
                    (CallFunction|AddStaticBlock (Math|Transform|MakeTransform (+ (Math|Vector|MakeVector (* (Variables|Dimensions|GetcurrentWidth) (Variables|Dimensions|GetmeshW)) (* (Variables|Dimensions|GetcurrentLength) (Variables|Dimensions|GetmeshL)) (* (Variables|Dimensions|GetcurrentHeight) (Variables|Dimensions|GetmeshH))) (Variables|Pivot|GetpivotPoint)) "0, 0, 0" "1,1,1"))
                    (else
                      ;[1 1 1] Add instanced block
                      (CallFunction|AddInstancedBlock (Math|Transform|MakeTransform (+ (Math|Vector|MakeVector (* (Variables|Dimensions|GetcurrentWidth) (Variables|Dimensions|GetmeshW)) (* (Variables|Dimensions|GetcurrentLength) (Variables|Dimensions|GetmeshL)) (* (Variables|Dimensions|GetcurrentHeight) (Variables|Dimensions|GetmeshH))) (Variables|Pivot|GetpivotPoint)) "0, 0, 0" "1,1,1")))))))))
        (:then_2
          ;[1 1 1] Set existing rotation
          (Variables|Movement|SetCurrentRotation (Transformation|GetWorldRotation (Variables|Transformation|GetRootComponent)))
          (if (Variables|Movement|GetIsMoving?)
            (Utilities|IsValid (Variables|Movement|GetPath)
              (:Is%20Valid
                (Variables|Default|SetTargetPath (Variables|/Game/Blueprints/Scene/BlockPath.BlockPath_C|GetPath (Variables|Movement|GetPath)))
                ;[1 1 1] Set spline length
                (Variables|Movement|SetSplineLength (Spline|GetSplineLength (Variables|Default|GetTargetPath)))
                ;[1 1 1] Set movement speed
                (Components|Timeline|SetPlayRate (Variables|Default|GetBlockMover) (/ 1.0 (Variables|Movement|GetMovementDuration)))
                ;[1 1 1] Set starting offset
                (Components|Timeline|SetNewTime (Variables|Default|GetBlockMover) (Variables|Movement|GetStartOffset))
                ;[1 1 1] Get spline rotation and location
                (CallFunction|InitMover))
              (:Is%20Not%20Valid
                (Variables|Movement|SetIsMoving? false)
                (Development|PrintString "WARNING: No valid spline path")))))))))

(fn AddInstancedBlock
  (params (transform :type Transform))
  (bind _instancedmeshcomponent (Variables|Object|GetInstancedMeshComponent))
  (bind _returnvalue (Components|InstancedStaticMesh|AddInstance _instancedmeshcomponent transform))
  (Rendering|Material|SetMaterial _instancedmeshcomponent _returnvalue (Variables|Object|GetMaterial))
  (if (Variables|Object|GetIsWalkable?)
    (Class|PrimitiveComponent|SetWalkableSlopeOverride _instancedmeshcomponent)
    (else
      (Class|PrimitiveComponent|SetWalkableSlopeOverride _instancedmeshcomponent (Utilities|Struct|MakeWalkableSlopeOverride "WalkableSlope_Unwalkable" 0.0)))))

(fn GetSplineDistance
  (params (MovementType :type ETimelineDirection%20Enum :default "Forward"))
  (switch Utilities|FlowControl|Switch|SwitchonETimelineDirection MovementType
    (:Forward
      (return (Math|Float|Lerp 0.0 (Variables|Movement|GetSplineLength) (Variables|Movement|GetMovementAlpha))))
    (:Backward
      (return (Math|Float|Lerp (Variables|Movement|GetSplineLength) 0.0 (Variables|Movement|GetMovementAlpha))))))

(fn AddStaticBlock
  (params (Transform :type Transform))
  (bind _returnvalue (AddComponent|AddStaticMeshComponent true Transform))
  (LocalVariables|SetcurrentMesh _returnvalue)
  (Transformation|AttachComponentToComponent (LocalVariables|GetcurrentMesh) (Variables|Object|GetblockRoot) "None" "KeepRelative" "KeepRelative" "KeepRelative" true)
  (Utilities|Array|Add (Variables|Object|GetBlocks) (LocalVariables|GetcurrentMesh))
  (Components|StaticMesh|SetStaticMesh (LocalVariables|GetcurrentMesh) (Variables|Object|GetStaticMesh))
  (Rendering|Material|SetMaterial (LocalVariables|GetcurrentMesh) 0 (Variables|Object|GetMaterial))
  (Transformation|SetRelativeTransform (LocalVariables|GetcurrentMesh) Transform false false)
  (if (Variables|Object|GetIsWalkable?)
    (Class|PrimitiveComponent|SetWalkableSlopeOverride (LocalVariables|GetcurrentMesh))
    (else
      (Class|PrimitiveComponent|SetWalkableSlopeOverride (LocalVariables|GetcurrentMesh) (Utilities|Struct|MakeWalkableSlopeOverride "WalkableSlope_Unwalkable" 0.0)))))

(fn GetFrameRotation
  (params (dt :type Float%20%28single-precision%29))
  (bind _rotationduration (Variables|Movement|GetRotationDuration))
  (Utilities|FlowControl|Sequence
    (:then_0
      (if (> (Math|Float|Absolute(Float) (.roll _rotationduration)) 0.0)
        (LocalVariables|Setx (/ 1.0 (.roll (Variables|Movement|GetRotationDuration)))))
      (if (> (Math|Float|Absolute(Float) (.pitch _rotationduration)) 0.0)
        (LocalVariables|Sety (/ 1.0 (.pitch (Variables|Movement|GetRotationDuration)))))
      (if (> (Math|Float|Absolute(Float) (.yaw _rotationduration)) 0.0)
        (LocalVariables|Setz (/ 1.0 (.yaw (Variables|Movement|GetRotationDuration))))))
    (:then_1
      (return (* (* (Math|Rotator|MakeRotator (LocalVariables|Getx) (LocalVariables|Gety) (LocalVariables|Getz)) dt) 3.6e+02)))))