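; AreaModifier is a box volume that temporarily changes how JUMP_Player moves while inside it.
; On begin overlap it caches and overrides whichever CharacterMovement properties are enabled by Custom flags: walkable floor angle, ground friction, jump velocity, air control and gravity scale.
; On end overlap it restores the cached values after an actor check.
; The construction script sizes the PhysicsModifier box from Range.
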(event OnComponentBeginOverlap(PhysicsModifier)
  (params (OverlappedComponent :type Primitive%20Component%20Object%20Reference) (OtherActor :type Actor%20Object%20Reference) (OtherComp :type Primitive%20Component%20Object%20Reference) (OtherBodyIndex :type Integer) (bFromSweep :type Boolean) (SweepResult :type Hit%20Result%20Structure%20%28by%20ref%29))
  (bind _asjump_player (Utilities|Casting|CastToJUMP_Player OtherActor))
  (Variables|Default|Setplayer _asjump_player)
  (if (Variables|Bools|GetCustomWalkableAngle)
    (Variables|Defaults|SetoldWalkableAngle (Class|CharacterMovementComponent|GetWalkableFloorAngle (Variables|/Script/Engine.Character|GetCharacterMovement (Variables|Default|Getplayer))))
    (Pawn|Components|CharacterMovement|SetWalkableFloorAngle (Variables|/Script/Engine.Character|GetCharacterMovement (Variables|Default|Getplayer)) (Variables|Vars|GetWalkableAngle)))
  (if (Variables|Bools|GetCustomGroundFriction)
    (Variables|Defaults|SetoldGroundFriction (Variables|/Script/Engine.CharacterMovementComponent|GetGroundFriction (Variables|/Script/Engine.Character|GetCharacterMovement (Variables|Default|Getplayer))))
    (Variables|/Script/Engine.CharacterMovementComponent|SetGroundFriction (Variables|/Script/Engine.Character|GetCharacterMovement (Variables|Default|Getplayer)) (Variables|Vars|GetgroundFriction)))
  (if (Variables|Bools|GetCustomJumpHeight)
    (Variables|Defaults|SetoldJumpSpeed (Variables|/Script/Engine.CharacterMovementComponent|GetJumpZVelocity (Variables|/Script/Engine.Character|GetCharacterMovement (Variables|Default|Getplayer))))
    (Variables|/Script/Engine.CharacterMovementComponent|SetJumpZVelocity (Variables|/Script/Engine.Character|GetCharacterMovement (Variables|Default|Getplayer)) (Variables|Vars|GetJumpSpeed)))
  (if (Variables|Bools|GetCustomAirControl)
    (Variables|Defaults|SetoldAirControl (Variables|/Script/Engine.CharacterMovementComponent|GetAirControl (Variables|/Script/Engine.Character|GetCharacterMovement (Variables|Default|Getplayer))))
    (Variables|/Script/Engine.CharacterMovementComponent|SetAirControl (Variables|/Script/Engine.Character|GetCharacterMovement (Variables|Default|Getplayer)) (Variables|Vars|GetAirControl)))
  (if (Variables|Bools|GetCustomGravity)
    (Variables|Defaults|SetoldGravityScale (Variables|/Script/Engine.CharacterMovementComponent|GetGravityScale (Variables|/Script/Engine.Character|GetCharacterMovement (Variables|Default|Getplayer))))
    (Variables|/Script/Engine.CharacterMovementComponent|SetGravityScale (Variables|/Script/Engine.Character|GetCharacterMovement (Variables|Default|Getplayer)) (Variables|Vars|GetgravityScale))))

(event OnComponentEndOverlap(PhysicsModifier)
  (params (OverlappedComponent :type Primitive%20Component%20Object%20Reference) (OtherActor :type Actor%20Object%20Reference) (OtherComp :type Primitive%20Component%20Object%20Reference) (OtherBodyIndex :type Integer))
  (if (== OtherActor 0)
    (if (Variables|Bools|GetCustomWalkableAngle)
      (Pawn|Components|CharacterMovement|SetWalkableFloorAngle (Variables|/Script/Engine.Character|GetCharacterMovement (Variables|Default|Getplayer)) (Variables|Defaults|GetoldWalkableAngle)))
    (if (Variables|Bools|GetCustomGroundFriction)
      (Variables|/Script/Engine.CharacterMovementComponent|SetGroundFriction (Variables|/Script/Engine.Character|GetCharacterMovement (Variables|Default|Getplayer)) (Variables|Defaults|GetoldGroundFriction)))
    (if (Variables|Bools|GetCustomJumpHeight)
      (Variables|/Script/Engine.CharacterMovementComponent|SetJumpZVelocity (Variables|/Script/Engine.Character|GetCharacterMovement (Variables|Default|Getplayer)) (Variables|Defaults|GetoldJumpSpeed)))
    (if (Variables|Bools|GetCustomAirControl)
      (Variables|/Script/Engine.CharacterMovementComponent|SetAirControl (Variables|/Script/Engine.Character|GetCharacterMovement (Variables|Default|Getplayer)) (Variables|Defaults|GetoldAirControl)))
    (if (Variables|Bools|GetCustomGravity)
      (Variables|/Script/Engine.CharacterMovementComponent|SetGravityScale (Variables|/Script/Engine.Character|GetCharacterMovement (Variables|Default|Getplayer)) (Variables|Defaults|GetoldGravityScale)))))

(event EventBeginPlay)

(event Collision|EventActorBeginOverlap
  (params (OtherActor :type Actor%20Object%20Reference)))

(event EventTick
  (params (DeltaSeconds :type Float%20%28single-precision%29)))

(fn ConstructionScript
  (Components|Box|SetBoxExtent (Variables|Default|GetPhysicsModifier) (Variables|BoxSettings|GetRange) true))