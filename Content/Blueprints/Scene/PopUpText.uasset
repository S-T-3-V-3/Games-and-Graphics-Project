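; PopUpText is a scene Blueprint that displays configurable text through a TextRender, set from its Text variable on BeginPlay.
; A TextArea overlap stores the JUMP_Player and sets IsActive, which is cleared when a JUMP_Player leaves.
; LookAtPlayer rotates the text toward that player's camera manager location, though nothing here calls it or reads IsActive.
; GetSteamRecord is an empty event.
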(event OnComponentBeginOverlap(TextArea)
  (params (OverlappedComponent :type Primitive%20Component%20Object%20Reference) (OtherActor :type Actor%20Object%20Reference) (OtherComp :type Primitive%20Component%20Object%20Reference) (OtherBodyIndex :type Integer) (bFromSweep :type Boolean) (SweepResult :type Hit%20Result%20Structure%20%28by%20ref%29))
  (bind _asjump_player (Utilities|Casting|CastToJUMP_Player OtherActor))
  (Variables|Default|SetisActive? true)
  (Variables|Default|SetPlayer _asjump_player))

(event OnComponentEndOverlap(TextArea)
  (params (OverlappedComponent :type Primitive%20Component%20Object%20Reference) (OtherActor :type Actor%20Object%20Reference) (OtherComp :type Primitive%20Component%20Object%20Reference) (OtherBodyIndex :type Integer))
  (Utilities|Casting|CastToJUMP_Player OtherActor)
  (Variables|Default|SetisActive? false))

(event Custom|LookAtPlayer
  (Transformation|SetWorldRotation (Variables|Default|GetTextRender) (Math|Rotator|FindLookatRotation (Transformation|GetWorldLocation (Variables|Default|GetTextRender)) (Transformation|GetWorldLocation (Variables|/Script/Engine.PlayerCameraManager|GetTransformComponent (Variables|/Script/Engine.PlayerController|GetPlayerCameraManager (Variables|/Game/Blueprints/JUMP_Player.JUMP_Player_C|GetOwningPlayer (Variables|Default|GetPlayer)))))) false false))

(event Custom|GetSteamRecord)

(event EventBeginPlay
  (Rendering|Components|TextRender|SetText (Variables|Default|GetTextRender) (Variables|Default|GetText)))

(event Collision|EventActorBeginOverlap
  (params (OtherActor :type Actor%20Object%20Reference)))

(event EventTick
  (params (DeltaSeconds :type Float%20%28single-precision%29)))

(fn ConstructionScript)