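; NeonBall is a scene actor with a ball component whose neon glow follows its speed.
; The construction script applies a dynamic instance of the Neon_BlackCyan material to the ball.
; Each tick, while speed is at or below MinSpeed, it scales EmissiveMultiplier from zero to one by speed over MinSpeed, dimming the glow as the ball slows.
; Above MinSpeed, the parameter is left unchanged.
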(event EventBeginPlay)

(event Collision|EventActorBeginOverlap
  (params (OtherActor :type Actor%20Object%20Reference)))

(event EventTick
  (params (DeltaSeconds :type Float%20%28single-precision%29))
  (bind _output_get (Variables|Default|SetSpeed (Math|Vector|VectorLength (Transformation|GetComponentVelocity (Variables|Default|GetBall)))))
  (if (not (> _output_get (Variables|Default|GetminSpeed)))
    (Rendering|Material|SetScalarParameterValue (Variables|Default|GetDynamicMaterial) "EmissiveMultiplier" (Math|Float|Lerp 0.0 1.0 (/ (Variables|Default|GetSpeed) (Variables|Default|GetminSpeed))) :!class /Script/Engine.MaterialInstanceDynamic)))

(fn ConstructionScript
  (bind _returnvalue (Rendering|Material|CreateDynamicMaterialInstance "/Game/Materials/Neon_BlackCyan.Neon_BlackCyan" "None" :!class /Script/Engine.KismetMaterialLibrary))
  (bind _output_get (Variables|Default|SetDynamicMaterial _returnvalue))
  (Rendering|Material|SetMaterial (Variables|Default|GetBall) 0 _output_get))