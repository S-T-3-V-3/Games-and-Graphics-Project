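; LevelManager runs one level of a jump game, handling player entry, exit, timed start and finish, and boundary respawns.
; On BeginPlay it registers itself with the start zone, end zone and map bounds, or prints an invalid-level error.
; Start and finish events drive the player's level tracker, while Compare_Results keeps the lowest score, updates the high-score text and alerts through the game mode.
; The construction script caches the respawn transform in LevelInfo.
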(event Custom|OnPlayerEntry
  (params (Player :type JUMP%20Controller%20Object%20Reference))
  (Default|EnterLevel Player (Variables|Default|GetLevelInfo)))

(event Custom|OnPlayerStart
  (params (Player :type JUMP%20Controller%20Object%20Reference))
  (bind _currentleveltracker (Variables|/Game/Blueprints/JUMP_Controller.JUMP_Controller_C|GetCurrentLevelTracker Player))
  (Utilities|IsValid _currentleveltracker
    (:Is%20Valid
      (Default|StartTimer _currentleveltracker))))

(event Custom|OnPlayerFinish
  (params (Player :type JUMP%20Controller%20Object%20Reference))
  (bind _currentleveltracker (Variables|/Game/Blueprints/JUMP_Controller.JUMP_Controller_C|GetCurrentLevelTracker Player))
  (Utilities|IsValid _currentleveltracker
    (:Is%20Valid
      (Default|EndTimer _currentleveltracker)
      (Default|OnLevelComplete _currentleveltracker self))))

(event Custom|OnPlayerExit
  (params (Player :type JUMP%20Controller%20Object%20Reference))
  (Default|ExitLevel Player))

(event Custom|Compare_Results
  (params (Best%20result :type Level%20Result%20Structure) (player%20name :type Text))
  (bind _levelinfo (Variables|Default|GetLevelInfo))
  (bind _levelinfo_2 (Variables|Default|GetLevelInfo))
  (bind (_levelindex _respawntransform _hasbeencompleted_ _bestresult) (Utilities|Struct|BreakLevelInfo _levelinfo))
  (bind (_levelindex_2 _respawntransform_2 _hasbeencompleted__2 _bestresult_2 _bestplayername) (Utilities|Struct|BreakLevelInfo _levelinfo_2))
  (bind (_score _scoredatetime _totalattempts) (Utilities|Struct|BreakLevelResult _bestresult_2))
  (if _hasbeencompleted_
    (if (< (.Score (Utilities|Struct|BreakLevelResult Best%20result)) (.score _bestresult))
      (Utilities|Struct|SetmembersinLevelInfo (Variables|Default|GetLevelInfo) Best%20result player%20name)
      (Default|UpdateHighScore (Variables|Default|GetHighScoreText) _bestresult_2 _bestplayername :!label _label)
      (bind _asjump_game_mode (Utilities|Casting|CastToJUMP_GameMode (Game|GetGameMode)))
      (Default|Alert _asjump_game_mode (Utilities|Text|FormatText "New High Score! 
{Player} completed Level {level} in {time} after {attempts} attempts." _bestplayername _levelindex_2 _score _totalattempts) "(R=0.964126,G=1.000000,B=0.000000,A=1.000000)"))
    (else
      (Utilities|Struct|SetmembersinLevelInfo (Variables|Default|GetLevelInfo) true Best%20result player%20name)
      (goto _label))))

(event Custom|OnPlayerHitBoundary
  (params (Player :type JUMP%20Controller%20Object%20Reference))
  (CallFunction|RespawnPlayer Player (Pawn|GetControlRotation Player :!class /Script/Engine.Controller)))

(event Custom|RespawnPlayer
  (params (Player :type JUMP%20Controller%20Object%20Reference) (CurrentControlRot :type Rotator))
  (bind _returnvalue (Pawn|GetControlRotation Player :!class /Script/Engine.Controller))
  (Default|Respawn Player)
  (Pawn|SetControlRotation Player (Math|Rotator|MakeRotator (.roll _returnvalue) (.pitch CurrentControlRot) (.yaw _returnvalue))))

(event EventBeginPlay
  ;[1 1 1] Check map validity
  (if (Math|Boolean|ANDBoolean (Utilities|IsValid (Variables|Default|GetRespawnPoint)) (Utilities|IsValid (Variables|Default|GetStartZone)) (Utilities|IsValid (Variables|Default|GetEndZone)) (Utilities|IsValid (Variables|Default|GetMapBounds)))
    ;[1 1 1] Set references
    (Variables|/Game/Blueprints/Scene/MapBounds.MapBounds_C|SetLevelManager (Variables|Default|GetMapBounds) self)
    (Variables|/Game/Blueprints/Scene/EndZone.EndZone_C|SetLevelManager (Variables|Default|GetEndZone) self)
    (Variables|/Game/Blueprints/Scene/StartZone.StartZone_C|SetLevelManager (Variables|Default|GetStartZone) self)
    (else
      (Development|PrintString (Utilities|String|ToString(Text) (Utilities|Text|FormatText "Level {LevelName} is invalid!" (.levelindex (Variables|Default|GetLevelInfo)))) true true "(R=1.000000,G=0.025630,B=0.000000,A=1.000000)" 2e+01))))

(event EventTick
  (params (DeltaSeconds :type Float%20%28single-precision%29)))

(fn ConstructionScript
  (bind _respawnpoint (Variables|Default|GetRespawnPoint))
  (Utilities|IsValid _respawnpoint
    (:Is%20Valid
      (Utilities|Struct|SetmembersinLevelInfo (Variables|Default|GetLevelInfo) (Transformation|GetWorldTransform (Variables|/Game/Blueprints/Scene/RespawnPoint.RespawnPoint_C|GetCapsule _respawnpoint))))))