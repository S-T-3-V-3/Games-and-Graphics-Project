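; MapBounds is a configurable boundary box that reacts when the first local player's JUMP_Player overlaps it.
; The construction script sizes and positions six faces from a Bounds vector, sets their outline visibility, and destroys any disabled faces.
; On overlap it notifies the LevelManager supplied through Init, or, without a valid one, calls ServerRespawn on the player's controller if MainArea is set.
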(event Custom|Init
  (params (LevelManager :type Level%20Manager%20Object%20Reference))
  (Variables|Default|SetLevelManager LevelManager))

(event Collision|EventActorBeginOverlap
  (params (OtherActor :type Actor%20Object%20Reference))
  (bind _asjump_player (Utilities|Casting|CastToJUMP_Player OtherActor))
  (if (== (Pawn|GetController _asjump_player) (Game|GetPlayerController 0))
    (Utilities|IsValid (Variables|Default|GetLevelManager)
      (:Is%20Valid
        (Default|OnPlayerHitBoundary (Variables|Default|GetLevelManager) (.AsJUMP%20Controller (Utilities|Casting|CastToJUMP_Controller (Game|GetPlayerController 0)))))
      (:Is%20Not%20Valid
        (if (Variables|Default|GetMainArea?)
          (Default|ServerRespawn (.AsJUMP%20Controller (Utilities|Casting|CastToJUMP_Controller (Game|GetPlayerController 0)))))))))

(fn ConstructionScript
  (bind _bounds (Variables|Default|GetBounds))
  (bind _bounds_2 (Variables|Default|GetBounds))
  (bind _bounds_3 (Variables|Default|GetBounds))
  (bind _bounds_4 (Variables|Default|GetBounds))
  (bind _bounds_5 (Variables|Default|GetBounds))
  (bind _bounds_6 (Variables|Default|GetBounds))
  (bind _returnvalue (/ _bounds 50))
  (bind _returnvalue_2 (/ _bounds_2 50))
  (bind _returnvalue_3 (/ _bounds_6 50))
  (Rendering|SetVisibility (Variables|Default|GetBack) (Variables|Default|GetShowOutline?) false)
  (Transformation|SetRelativeScale3D (Variables|Default|GetFront) (Math|Vector|MakeVector (.z _returnvalue) (.y _returnvalue) 1.0))
  (Transformation|SetRelativeScale3D (Variables|Default|GetTop) (Math|Vector|MakeVector (.x _returnvalue_2) (.y _returnvalue_2) 1.0))
  (Transformation|SetRelativeScale3D (Variables|Default|GetLeft) (Math|Vector|MakeVector (.z _returnvalue_3) (.x _returnvalue_3) 1.0))
  (Transformation|SetRelativeLocation (Variables|Default|GetFront) (Math|Vector|MakeVector (.x _bounds_4) 0.0 0.0) false false)
  (Transformation|SetRelativeLocation (Variables|Default|GetBack) (Math|Vector|MakeVector (* -1 (.x _bounds_4)) 0.0 0.0) false false)
  (Transformation|SetRelativeLocation (Variables|Default|GetTop) (Math|Vector|MakeVector 0.0 0.0 (.z _bounds_5)) false false)
  (Transformation|SetRelativeLocation (Variables|Default|GetBottom) (Math|Vector|MakeVector 0.0 0.0 (* -1 (.z _bounds_5))) false false)
  (Transformation|SetRelativeLocation (Variables|Default|GetRight) (Math|Vector|MakeVector 0.0 (.y _bounds_3) 0.0) false false)
  (Transformation|SetRelativeLocation (Variables|Default|GetLeft) (Math|Vector|MakeVector 0.0 (* -1 (.y _bounds_3)) 0.0) false false)
  (Utilities|FlowControl|Sequence
    (:then_0
      (if (Variables|Default|GetDisableFront)
        (Components|DestroyComponent (Variables|Default|GetFront))))
    (:then_1
      (if (Variables|Default|GetDisableBack)
        (Components|DestroyComponent (Variables|Default|GetBack))))
    (:then_2
      (if (Variables|Default|GetDisableTop)
        (Components|DestroyComponent (Variables|Default|GetTop))))
    (:then_3
      (if (Variables|Default|GetDisableLeft)
        (Components|DestroyComponent (Variables|Default|GetLeft))))
    (:then_4
      (if (Variables|Default|GetDisableRight)
        (Components|DestroyComponent (Variables|Default|GetRight))))
    (:then_5
      (if (Variables|Default|GetDisableBottom)
        (Components|DestroyComponent (Variables|Default|GetBottom))))))