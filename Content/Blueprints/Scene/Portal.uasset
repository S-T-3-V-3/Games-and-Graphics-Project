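; Linked portal actor that shows the view through its partner portal and seamlessly teleports the local player across.
; Each update mirrors the player camera onto the partner's scene capture, whose render target feeds this screen through a dynamic material.
; A clip plane flips with the camera's side.
; Overlap records the entry side, and crossing the plane triggers teleport with a rotation offset, notifying the connected level for map start/end portals.
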(event OnComponentBeginOverlap(Box)
  (params (OverlappedComponent :type Primitive%20Component%20Object%20Reference) (OtherActor :type Actor%20Object%20Reference) (OtherComp :type Primitive%20Component%20Object%20Reference) (OtherBodyIndex :type Integer) (bFromSweep :type Boolean) (SweepResult :type Hit%20Result%20Structure%20%28by%20ref%29))
  ;[1 1 1] Check if player is overlapped
  (bind _asjump_player (Utilities|Casting|CastToJUMP_Player OtherActor))
  (if (== (Pawn|GetController _asjump_player) (Game|GetPlayerController 0))
    (Variables|Default|SetisPlayerHere? true)
    (Utilities|FlowControl|Sequence
      (:then_0
        ;[1 1 1] Set Player Portal Location
        (bind (_x _success_) (CallFunction|GetPlayerRelativeXLoc))
        (if (and (> _x 0.0) _success_)
          (Variables|Default|SetPlayerLocation "NewEnumerator0")
          (else
            (Variables|Default|SetPlayerLocation "NewEnumerator1")))))))

(event OnComponentEndOverlap(Box)
  (params (OverlappedComponent :type Primitive%20Component%20Object%20Reference) (OtherActor :type Actor%20Object%20Reference) (OtherComp :type Primitive%20Component%20Object%20Reference) (OtherBodyIndex :type Integer))
  ;[1 1 1] Check if player is overlapped
  (bind _asjump_player (Utilities|Casting|CastToJUMP_Player OtherActor))
  (if (== (Pawn|GetController _asjump_player) (Game|GetPlayerController 0))
    (Variables|Default|SetisPlayerHere? false)))

(event Custom|UpdateOtherCamera
  (bind _otherportal (Variables|Default|GetotherPortal))
  (bind _asportal (Utilities|Casting|CastToPortal _otherportal))
  (bind _portalcamera (Variables|Portal_C|GetPortalCamera _asportal))
  ;[1 1 1] Update camera transform
  (bind _transform (CallFunction|GetPlayerCameraTransform))
  (Transformation|SetRelativeLocation _portalcamera (.location (Math|Transform|MakeRelativeTransform _transform (Transformation|GetWorldTransform (Variables|Default|Getroot)))) false false)
  (Transformation|SetRelativeRotation _portalcamera (.rotation (Math|Transform|MakeRelativeTransform _transform (Transformation|GetWorldTransform (Variables|Default|Getroot)))) false false))

(event Custom|UpdateClippingPlane
  (bind _otherportal (Variables|Default|GetotherPortal))
  (bind _otherportal_2 (Variables|Default|GetotherPortal))
  (bind _portalnormalmultiplier (Variables|Default|GetportalNormalMultiplier))
  (bind _asportal (Utilities|Casting|CastToPortal _otherportal_2))
  (bind _asportal_2 (Utilities|Casting|CastToPortal _otherportal))
  (bind _portalcamera (Variables|Portal_C|GetPortalCamera _asportal))
  (bind _root (Variables|Portal_C|Getroot _asportal_2))
  (bind _returnvalue (Math|Vector|GetForwardVector _root))
  (bind _returnvalue_2 (* _returnvalue _portalnormalmultiplier))
  ;[1 1 1] Clipping plane calculation
  (Variables|/Script/Engine.SceneCaptureComponent2D|SetClipPlaneNormal _portalcamera _returnvalue_2)
  (Variables|/Script/Engine.SceneCaptureComponent2D|SetClipPlaneBase _portalcamera (+ (Transformation|GetWorldLocation _root) (* _returnvalue_2 -2e+01))))

(event Custom|UpdateDisplayNormal
  ;[1 1 1] Get player camera location, toggle clipping plane and flip normals where necessary
  (bind _x_loc (CallFunction|GetPlayerCameraRelativeXLoc))
  (if (> _x_loc 0.0)
    (CallFunction|SetNormal -1)
    (else
      (CallFunction|SetNormal 1))))

(event Custom|CheckScreenVisibility
  ;[1 1 1] Visibility
  (bind _x_loc (CallFunction|GetPlayerCameraRelativeXLoc))
  (bind _x (CallFunction|GetPlayerRelativeXLoc))
  (Rendering|SetVisibility (Variables|Default|GetportalScreen) (not (Class|KismetMathLibrary|XORBoolean (> _x 0.0) (> _x_loc 0.0))) false))

(event Custom|RequiresTeleport?
  (bind _returnvalue (Game|GetPlayerController 0))
  (bind _distanceoffset (Variables|Default|GetDistanceOffset))
  (bind _otherportal (Variables|Default|GetotherPortal))
  (bind _connectedlevel (Variables|Default|GetConnectedLevel))
  (bind _asjump_controller (Utilities|Casting|CastToJUMP_Controller _returnvalue))
  (bind _teleportlocationcomponent (Variables|/Script/JUMP.JumpPortal|GetTeleportLocationComponent _otherportal))
  ;[1 1 1] Check if player requires teleport
  (if (Variables|Default|GetisPlayerHere?)
    (bind _x (CallFunction|GetPlayerRelativeXLoc))
    (switch Utilities|FlowControl|Switch|SwitchonPlayerPortalLocation (Variables|Default|GetPlayerLocation)
      (:NewEnumerator0
        (if (<= _x (* -1 _distanceoffset))
          (bind _playerref (Default|GetPlayerRef (.AsJUMP%20Controller (Utilities|Casting|CastToJUMP_Controller (Game|GetPlayerController 0))) :!label _label))
          (Transformation|SetRelativeTransform _teleportlocationcomponent (Math|Transform|MakeRelativeTransform (Transformation|GetWorldTransform (Variables|/Script/Engine.Actor|GetRootComponent _playerref)) (Transformation|GetWorldTransform (Variables|Default|Getroot))) false false)
          (Utilities|FlowControl|Sequence
            (:then_0
              (switch Utilities|FlowControl|Switch|SwitchonPortalType (Variables|Default|GetType)
                (:NewEnumerator1
                  (Default|OnPlayerEntry _connectedlevel _asjump_controller))
                (:NewEnumerator2
                  (Default|OnPlayerExit _connectedlevel _asjump_controller))))
            (:then_1
              ;[1 1 1] Teleport Player
              (bind _returnvalue_2 (CallFunction|GetPlayerCameraRelativeRotation))
              (bind _playerref_2 (Default|GetPlayerRef (.AsJUMP%20Controller (Utilities|Casting|CastToJUMP_Controller (Game|GetPlayerController 0)))))
              (Default|Teleport _playerref_2 (Transformation|GetWorldTransform _teleportlocationcomponent) _returnvalue_2 (Variables|Default|GetrotationDifference))
              (Class|JUMPFunctionLibrary|ForceCameraUpdate)
              (CallFunction|UpdateDisplayNormal (.AsPortal (Utilities|Casting|CastToPortal (Variables|Default|GetotherPortal))))))))
      (:NewEnumerator1
        (if (>= _x _distanceoffset)
          (goto _label))))))

(event Custom|GetPortalRotationDifference
  (bind _root (Variables|Default|Getroot))
  (bind _otherportal (Variables|Default|GetotherPortal))
  (bind _returnvalue (Transformation|GetWorldRotation _root))
  (bind _rootcomponent (Variables|/Script/Engine.Actor|GetRootComponent _otherportal))
  (bind _returnvalue_2 (Transformation|GetWorldRotation _rootcomponent))
  ;[1 1 1] Portal Rotation Difference
  (Variables|Default|SetrotationDifference (Math|Rotator|MakeRotator (- (.roll _returnvalue_2) (.roll _returnvalue)) (- (.pitch _returnvalue_2) (.pitch _returnvalue)) (- (.yaw _returnvalue_2) (.yaw _returnvalue)))))

(event EventOnActiveStateChanged
  (params (isActive :type Boolean))
  (Rendering|SetVisibility (Variables|Default|GetportalScreen) isActive false)
  (CallFunction|CheckScreenVisibility))

(event EventOnUpdate
  ;[1 1 1] Update
  (CallFunction|GetPortalRotationDifference)
  (CallFunction|UpdateOtherCamera)
  (CallFunction|CheckScreenVisibility)
  (CallFunction|UpdateDisplayNormal)
  (CallFunction|UpdateClippingPlane)
  (CallFunction|RequiresTeleport?))

(event EventOnBegin
  (bind _otherportal (Variables|Default|GetotherPortal))
  ;[0 0.000306 1] Initialize
  ;;[1 1 1] Hide both portal screens from render view
  (Variables|Default|SetThisCamera (Variables|Default|GetPortalCamera))
  (Utilities|FlowControl|Delay 0.2)
  (Class|JumpPortal|Init)
  (Utilities|IsValid (Variables|Default|GetotherPortal)
    (:Is%20Valid
      (Variables|Default|SetisInitialized true)
      (Class|SceneCaptureComponent|HideComponent (Variables|Default|GetPortalCamera) (Variables|Default|GetArrow))
      (Class|SceneCaptureComponent|HideComponent (Variables|Default|GetPortalCamera) (Variables|Default|GetportalScreen))
      (Class|SceneCaptureComponent|HideComponent (Variables|Default|GetPortalCamera) (Variables|Portal_C|GetportalScreen (.AsPortal (Utilities|Casting|CastToPortal (Variables|Default|GetotherPortal)))))
      ;;[1 1 1] Tell our screen to display the rendered material of the connected portal
      (Rendering|Material|SetMaterial (Variables|Default|GetportalScreen) 0 (Variables|Portal_C|GetportalMaterial (.AsPortal (Utilities|Casting|CastToPortal (Variables|Default|GetotherPortal)))))
      (Variables|Default|SetOtherCamera (Variables|/Script/JUMP.JumpPortal|GetThisCamera _otherportal))
      (if (not (Variables|/Script/JUMP.JumpPortal|GetisInitialized _otherportal))
        (Class|JumpPortal|OnBegin)))
    (:Is%20Not%20Valid
      ;;[1 1 1] Portal is not linked - disable screen and turn frame red
      (Rendering|SetVisibility (Variables|Default|GetportalScreen) false false)
      (Rendering|Material|SetMaterial (Variables|Default|GetportalFrame) 0 "/Game/Materials/Neon_BlackRed.Neon_BlackRed"))))

(fn ConstructionScript
  (bind _textrender (Variables|Default|GetTextRender))
  (Variables|Default|SetThisCamera (Variables|Default|GetPortalCamera))
  (Variables|Default|SetTeleportLocationComponent (Variables|Default|GetteleportLocation))
  (Rendering|Components|TextRender|SetText _textrender (Variables|Default|GetPortalText_0))
  (Rendering|Components|TextRender|SetWorldSize _textrender (Variables|Default|GetTextSize))
  ;[1 1 1] Create texture target for camera to render to
  (bind _returnvalue (Rendering|CreateRenderTarget2D 1920 1080 "RTF_RGBA16f"))
  (bind _output_get (Variables|Default|SetCameraRenderTarget _returnvalue))
  (Variables|/Script/Engine.SceneCaptureComponent2D|SetTextureTarget (Variables|Default|GetPortalCamera) _output_get)
  ;[1 1 1] Create instance of render target material, pass through the camera view to it
  (bind _returnvalue_2 (Rendering|Material|CreateDynamicMaterialInstance "/Game/Materials/portalRenderTargetMat.portalRenderTargetMat" "portalMaterial" :!class /Script/Engine.KismetMaterialLibrary))
  (bind _output_get_2 (Variables|Default|SetportalMaterial _returnvalue_2))
  (Rendering|Material|SetTextureParameterValue _output_get_2 "targetMaterial" (Variables|Default|GetCameraRenderTarget)))

(fn SetNormal
  (params (normal :type Integer))
  (if (== (Variables|Default|GetportalNormalMultiplier) normal)
    (return false)
    (else
      (Variables|Default|SetportalNormalMultiplier normal)
      (return true))))

(fn GetPlayerCameraTransform
  (return (Transformation|GetWorldTransform (Variables|/Script/Engine.PlayerCameraManager|GetTransformComponent (Variables|/Script/Engine.PlayerController|GetPlayerCameraManager (.AsJUMP%20Controller (Utilities|Casting|CastToJUMP_Controller (Game|GetPlayerController 0))))))))

(fn GetPlayerCameraRelativeXLoc
  (bind _transform (CallFunction|GetPlayerCameraTransform))
  (return (.X (Math|Vector|BreakVector (.location (Math|Transform|MakeRelativeTransform _transform (Transformation|GetWorldTransform (Variables|Default|Getroot))))))))

(fn GetPlayerRelativeLoc
  (bind (_playerref _success) (Default|GetPlayerRef (.AsJUMP%20Controller (Utilities|Casting|CastToJUMP_Controller (Game|GetPlayerController 0)))))
  (if _success
    (return (.location (Math|Transform|MakeRelativeTransform (Transformation|GetWorldTransform (Variables|/Script/Engine.Character|GetCapsuleComponent _playerref)) (Transformation|GetWorldTransform (Variables|Default|Getroot)))) true)
    (else
      (return "0, 0, 0" false))))

(fn GetPlayerRelativeXLoc
  (bind _returnvalue (Game|GetPlayerController 0))
  (bind _asjump_controller (Utilities|Casting|CastToJUMP_Controller _returnvalue))
  (bind _returnvalue_2 (Pawn|GetControlledPawn _asjump_controller))
  (bind _asjump_character (Utilities|Casting|CastToJumpCharacter _returnvalue_2))
  (bind _capsulecomponent (Variables|/Script/Engine.Character|GetCapsuleComponent _asjump_character))
  (Utilities|IsValid _capsulecomponent
    (:Is%20Valid
      (return (.x (.location (Math|Transform|MakeRelativeTransform (Transformation|GetWorldTransform _capsulecomponent) (Transformation|GetWorldTransform (Variables|Default|Getroot))))) true))
    (:Is%20Not%20Valid
      (return 0.0 false))))

(fn GetPlayerCameraRelativeRotation
  (bind (_playerref _success) (Default|GetPlayerRef (.AsJUMP%20Controller (Utilities|Casting|CastToJUMP_Controller (Game|GetPlayerController 0)))))
  (if _success
    (return (Math|Rotator|MakeRotator (.roll (Pawn|GetControlRotation _playerref :!class /Script/Engine.Pawn)) (.pitch (Pawn|GetControlRotation _playerref :!class /Script/Engine.Pawn)) (+ (- (.yaw (Transformation|GetWorldRotation (Variables|/Script/Engine.Actor|GetRootComponent (Variables|Default|GetotherPortal)))) (.yaw (Transformation|GetWorldRotation (Variables|Default|Getroot)))) (.yaw (Pawn|GetControlRotation _playerref :!class /Script/Engine.Pawn)))))
    (else
      (return "0, 0, 0"))))

(fn GetPlayerCameraRelativeLoc
  (bind _transform (CallFunction|GetPlayerCameraTransform))
  (return (.location (Math|Transform|MakeRelativeTransform _transform (Transformation|GetWorldTransform (Variables|Default|Getroot))))))