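; Configurable level actor that can ping-pong between Start and End while spinning, with optional launch and kill flags.
; The construction script sets up colored endpoint previews, direction arrows, a slightly enlarged launch hitbox, and the offset or reversed spawn point.
; Tick moves it along the normalized direction, flipping at the endpoints by comparing only the first differing axis.
; Kill and launch hit handlers are empty; the cooldown-gated impulse logic is disconnected.
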(event OnComponentHit(LaunchHitbox)
  (params (HitComponent :type Primitive%20Component%20Object%20Reference) (OtherActor :type Actor%20Object%20Reference) (OtherComp :type Primitive%20Component%20Object%20Reference) (NormalImpulse :type Vector :default "0, 0, 0") (Hit :type Hit%20Result%20Structure%20%28by%20ref%29))
  ;[1 1 1] Launch Hitbox
  (if (Variables|Settings|GetLaunch)
    _))

(event Custom|isMoving
  (bind _start (Variables|Movement|GetStart))
  (bind _end (Variables|Movement|GetEnd))
  ;[1 1 1] Is Moving
  (if (Variables|Settings|GetMoving)
    (Rendering|SetVisibility (Variables|Default|GetEndLocation) true false)
    (Rendering|SetVisibility (Variables|Default|GetStartLocation) true false)
    (Variables|Default|SetDirection (Math|Vector|GetUnitDirection(Vector) (Variables|Movement|GetStart) (Variables|Movement|GetEnd)))
    (Variables|Default|SetDistance (Math|Float|Sqrt (+ (Math|Float|Square (- (.x _end) (.x _start))) (Math|Float|Square (- (.y _end) (.y _start))) (Math|Float|Square (- (.z _end) (.z _start))))))
    (if (== (.x (Variables|Movement|GetStart)) (.x (Variables|Movement|GetEnd)))
      (if (== (.y (Variables|Movement|GetStart)) (.y (Variables|Movement|GetEnd)))
        (if (== (.z (Variables|Movement|GetStart)) (.z (Variables|Movement|GetEnd)))
          _
          (else
            (Variables|Default|SetaxisMovement 2)
            (Variables|Default|SetstartPos (.z (Variables|Movement|GetStart)))
            (Variables|Default|SetendPos (.z (Variables|Movement|GetEnd)))))
        (else
          (Variables|Default|SetaxisMovement 1)
          (Variables|Default|SetstartPos (.y (Variables|Movement|GetStart)))
          (Variables|Default|SetendPos (.y (Variables|Movement|GetEnd)))))
      (else
        (Variables|Default|SetaxisMovement 0)
        (Variables|Default|SetstartPos (.x (Variables|Movement|GetStart)))
        (Variables|Default|SetendPos (.x (Variables|Movement|GetEnd)))))
    (if (< (Variables|Default|GetendPos) (Variables|Default|GetstartPos))
      (Variables|Default|Setnegative true))
    (if (Math|Vector|Equal(Vector) (Variables|Movement|GetCurrent) (Variables|Movement|GetStart) 0.0001)
      (Rendering|SetVisibility (Variables|Default|GetStartLocation) false false))
    (if (Math|Vector|Equal(Vector) (Variables|Movement|GetCurrent) (Variables|Movement|GetEnd) 0.0001)
      (Rendering|SetVisibility (Variables|Default|GetEndLocation) false false))))

(event Custom|setSpawnPoint
  ;[1 1 1] Set Spawn Point
  (if (> (Variables|Movement|GetStarting%20Offset%20%28%25%29) 0.0)
    (Variables|Movement|SetCurrent (+ (Variables|Movement|GetStart) (* (Variables|Default|GetDirection) (* (/ (Variables|Movement|GetStarting%20Offset%20%28%25%29) 1e+02) (Variables|Default|GetDistance)))))
    (else
      (Variables|Movement|SetCurrent (Variables|Movement|GetStart))))
  (if (Variables|Movement|GetReverse)
    (Variables|Default|Setnegative true))
  (Transformation|SetRelativeLocation (Variables|Default|GetActor) (Variables|Movement|GetCurrent) false false)
  (if (Variables|Movement|GetReverse)
    (if (not (Math|Vector|Equal(Vector) (Variables|Movement|GetCurrent) (Variables|Movement|GetStart) 0.0001))
      (Rendering|SetVisibility (Variables|Default|GetMovementDirection) true false)
      (Transformation|SetWorldRotation (Variables|Default|GetMovementDirection) (Math|Rotator|FindLookatRotation (Variables|Movement|GetCurrent) (Variables|Movement|GetStart)) false false))
    (elif (not (Math|Vector|Equal(Vector) (Variables|Movement|GetCurrent) (Variables|Movement|GetStart) 0.0001))
      (Rendering|SetVisibility (Variables|Default|GetMovementDirection) true false)
      (Transformation|SetWorldRotation (Variables|Default|GetMovementDirection) (Math|Rotator|FindLookatRotation (Variables|Movement|GetCurrent) (Variables|Movement|GetEnd)) false false))))

(event Custom|isReversed
  ;[1 1 1] IsReversed
  (if (Variables|Movement|GetReverse)
    (Variables|Default|Setended true)))

(event Custom|isLaunching
  (bind _actor (Variables|Default|GetActor))
  (bind _returnvalue (Transformation|GetWorldScale _actor))
  ;[1 1 1] IsLaunching
  (if (Variables|Settings|GetLaunch)
    (Rendering|SetVisibility (Variables|Default|GetLaunchDirectionArrow) true false)
    (Rendering|SetVisibility (Variables|Default|GetLaunchHitbox) true false)
    (if (< (.x _returnvalue) 1.0)
      (Variables|Default|SetscaleX (+ (/ (.x _returnvalue) 3e+01) (.x _returnvalue)))
      (else
        (Variables|Default|SetscaleX (+ (.x _returnvalue) 0.01))))
    (if (< (.y _returnvalue) 1.0)
      (Variables|Default|SetscaleY (+ (/ (.y _returnvalue) 3e+01) (.y _returnvalue)))
      (else
        (Variables|Default|SetscaleY (+ (.y _returnvalue) 0.01))))
    (if (< (.z _returnvalue) 1.0)
      (Variables|Default|SetscaleZ (+ (/ (.z _returnvalue) 3e+01) (.z _returnvalue)))
      (else
        (Variables|Default|SetscaleZ (+ (.z _returnvalue) 0.01))))
    (Transformation|SetWorldScale3D (Variables|Default|GetLaunchHitbox) (Math|Vector|MakeVector (Variables|Default|GetscaleX) (Variables|Default|GetscaleY) (Variables|Default|GetscaleZ)))
    (Transformation|SetWorldRotation (Variables|Default|GetLaunchDirectionArrow) (Variables|Launch|GetLaunchDirection) false false)))

(event Custom|doMovement
  (params (dt :type Float%20%28single-precision%29))
  (bind _move_speed (Variables|Movement|GetMove%20Speed))
  (bind _direction (Variables|Default|GetDirection))
  (bind _returnvalue (Math|Vector|Normalize _direction))
  (bind _returnvalue_2 (* dt _move_speed))
  (bind _returnvalue_3 (* _returnvalue _returnvalue_2))
  ;[1 1 1] Do Movement
  (if (Variables|Default|Getended)
    (Variables|Movement|SetCurrent (- (Variables|Movement|GetCurrent) _returnvalue_3))
    (else
      (Variables|Movement|SetCurrent (+ (Variables|Movement|GetCurrent) _returnvalue_3))))
  (Transformation|SetRelativeLocation (Variables|Default|GetActor) (Variables|Movement|GetCurrent) false false)
  (Transformation|AddWorldRotation (Variables|Default|GetActor) (* (Variables|Movement|GetRotation%20Speed) dt) false false)
  (switch int (Variables|Default|GetaxisMovement)
    (:0
      (Variables|Default|SetcurrentPos (.x (Variables|Movement|GetCurrent))))
    (:1
      (Variables|Default|SetcurrentPos (.y (Variables|Movement|GetCurrent))))
    (:2
      (Variables|Default|SetcurrentPos (.z (Variables|Movement|GetCurrent)))))
  (if (Variables|Default|Getnegative)
    (if (< (Variables|Default|GetcurrentPos) (Variables|Default|GetendPos))
      (Variables|Default|Setended true)
      (elif (>= (Variables|Default|GetcurrentPos) (Variables|Default|GetstartPos))
        (Variables|Default|Setended false)))
    (elif (> (Variables|Default|GetcurrentPos) (Variables|Default|GetendPos))
      (Variables|Default|Setended true)
      (elif (<= (Variables|Default|GetcurrentPos) (Variables|Default|GetstartPos))
        (Variables|Default|Setended false)))))

(event Custom|setEndpoints
  ;[1 1 1] Set Endpoints
  (Transformation|SetRelativeLocation (Variables|Default|GetStartLocation) (Variables|Movement|GetStart) false false)
  (Transformation|SetRelativeLocation (Variables|Default|GetEndLocation) (Variables|Movement|GetEnd) false false))

(event EventTick
  (params (DeltaSeconds :type Float%20%28single-precision%29))
  ;[1 1 1] Tick
  (if (Variables|Settings|GetMoving)
    (CallFunction|DoMovement DeltaSeconds))
  (if (> (Variables|Default|GetLaunchCooldownTimer) 0.0)
    (Variables|Default|SetLaunchCooldownTimer (- (Variables|Default|GetLaunchCooldownTimer) DeltaSeconds))))

(event Collision|EventHit
  (params (MyComp :type Primitive%20Component%20Object%20Reference) (Other :type Actor%20Object%20Reference) (OtherComp :type Primitive%20Component%20Object%20Reference) (bSelfMoved :type Boolean) (HitLocation :type Vector :default "0, 0, 0") (HitNormal :type Vector :default "0, 0, 0") (NormalImpulse :type Vector :default "0, 0, 0") (Hit :type Hit%20Result%20Structure%20%28by%20ref%29))
  ;[1 1 1] Kill Hitbox
  (if (Variables|Settings|GetKill)
    _))

(fn ConstructionScript
  (Components|StaticMesh|SetStaticMesh (Variables|Default|GetActor) (Variables|Settings|GetActor%20Mesh))
  (Components|StaticMesh|SetStaticMesh (Variables|Default|GetStartLocation) (Variables|Settings|GetActor%20Mesh))
  (Components|StaticMesh|SetStaticMesh (Variables|Default|GetEndLocation) (Variables|Settings|GetActor%20Mesh))
  (Components|StaticMesh|SetStaticMesh (Variables|Default|GetLaunchHitbox) (Variables|Settings|GetActor%20Mesh))
  (Rendering|Material|SetMaterial (Variables|Default|GetLaunchHitbox) 0 "/Game/Materials/Green.Green")
  (Rendering|Material|SetMaterial (Variables|Default|GetStartLocation) 0 "/Game/Materials/Blue.Blue")
  (Rendering|Material|SetMaterial (Variables|Default|GetEndLocation) 0 "/Game/Materials/Red.Red")
  (CallFunction|IsMoving)
  (CallFunction|IsLaunching)
  (CallFunction|IsReversed)
  (CallFunction|SetEndpoints)
  (CallFunction|SetSpawnPoint))