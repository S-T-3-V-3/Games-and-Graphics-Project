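; An in-level high score display that shows the best player's name, time in seconds and number of attempts.
; UpdateHighScore stores the new score and name, then GetServerHighScore passes the stored values to LocalUpdateScores, which formats and sets the text once a score exists.
; The construction script registers the display with LevelManager as its HighScoreText.
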(event Custom|LocalUpdateScores
  (params (BestScore :type Level%20Result%20Structure) (BestPlayerName :type Text) (isSet? :type Boolean))
  (if isSet?
    (Rendering|Components|TextRender|SetText (Variables|Default|GetPlayerName) BestPlayerName)
    (Rendering|Components|TextRender|SetText (Variables|Default|GetBest%20Time) (Utilities|Text|FormatText "{time}s" (.score BestScore)))
    (Rendering|Components|TextRender|SetText (Variables|Default|GetNumAttempts) (Utilities|Text|FormatText "{attempts} attempts" (.totalattempts BestScore)))))

(event Custom|UpdateHighScore
  (params (PlayerScore :type Level%20Result%20Structure) (PlayerName :type Text))
  (Variables|Default|SetisScoreSet? true)
  (Variables|Default|SetBestScore PlayerScore)
  (Variables|Default|SetBestPlayerName PlayerName)
  (CallFunction|GetServerHighScore))

(event Custom|GetServerHighScore
  (CallFunction|LocalUpdateScores (Variables|Default|GetBestScore) (Variables|Default|GetBestPlayerName) (Variables|Default|GetisScoreSet?)))

(event Collision|EventActorBeginOverlap
  (params (OtherActor :type Actor%20Object%20Reference)))

(event EventTick
  (params (DeltaSeconds :type Float%20%28single-precision%29)))

(fn ConstructionScript
  (Variables|/Game/Blueprints/Scene/LevelManager.LevelManager_C|SetHighScoreText (Variables|Default|GetLevelManager) self))