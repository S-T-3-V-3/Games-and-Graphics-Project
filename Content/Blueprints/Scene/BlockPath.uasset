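; BlockPath is a scene actor that provides an editable spline path with a configurable number of points.
; Its construction script rebuilds the Path spline only when the point count differs from NumPoints, placing evenly spaced points along local X at DefaultPointSpacing.
; Manual point edits therefore survive reconstruction as long as the count stays the same.
; It has no runtime logic; all event nodes are unused stubs.
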(event EventBeginPlay)

(event Collision|EventActorBeginOverlap
  (params (OtherActor :type Actor%20Object%20Reference)))

(event EventTick
  (params (DeltaSeconds :type Float%20%28single-precision%29)))

(fn ConstructionScript
  (if (!= (Spline|GetNumberOfSplinePoints (Variables|Default|GetPath)) (Variables|Default|GetNumPoints))
    (Spline|ClearSplinePoints (Variables|Default|GetPath) true)
    (Utilities|Array|Clear (LocalVariables|GetSpline%20Points))
    (for _index (range 0 (- (Variables|Default|GetNumPoints) 1))
      (Utilities|Array|Add (LocalVariables|GetSpline%20Points) (Math|Vector|MakeVector (Math|Conversions|ToFloat(Integer) (* _index (Variables|Default|GetDefaultPointSpacing))) 0.0 0.0)))
    (Spline|SetSplinePoints (Variables|Default|GetPath) (LocalVariables|GetSpline%20Points) "Local" true)))