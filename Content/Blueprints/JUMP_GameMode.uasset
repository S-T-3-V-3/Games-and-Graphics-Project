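; Game mode for JUMP that manages player joins and departures, spawning, respawning, chat and server alerts.
; On authority, PostLogin registers each controller, caches LevelManagers for high-score checks, and loads the player, retrying every half second before spawning and possessing a JUMP_Player.
; Spawns pick a random PlayerStart, or a tutorial RespawnPoint if the tutorial is unfinished.
; Chat, alerts and leave notices are relayed to every tracked controller.
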(event Custom|NewMessage
  (params (PlayerName :type String) (Message :type Text))
  ;[1 1 1] Chat
  (for _array_element (Variables|Default|GetAllPlayerControllers)
    (bind _asjump_controller (Utilities|Casting|CastToJUMP_Controller _array_element))
    (Default|ReceiveMessage _asjump_controller PlayerName Message)))

(event Custom|GetLevelManagers
  (bind _outactors (Actor|GetAllActorsOfClass "/Game/Blueprints/Scene/LevelManager.LevelManager_C"))
  (Variables|Default|SetLevelManagers _outactors))

(event Custom|UpdateClientPlayerList
  ;[1 0.3333 0.3432] Update player UI panels
)

(event Custom|RespanPlayer
  (params (PlayerController :type JUMP%20Controller%20Object%20Reference) (RespawnTransform :type Transform))
  (bind _returnvalue (Pawn|GetControlledPawn PlayerController))
  ;[1 0.7467 0.5294] Respawn a player
  (Utilities|IsValid _returnvalue
    (:Is%20Valid
      (Actor|DestroyActor _returnvalue))
    (:Is%20Not%20Valid
      _))
  (bind _returnvalue_2 (Game|SpawnActorfromClass "/Game/Blueprints/JUMP_Player.JUMP_Player_C" RespawnTransform "AdjustIfPossibleButAlwaysSpawn" PlayerController PlayerController 0))
  (Pawn|Possess PlayerController _returnvalue_2)
  (Default|SetLocalOwningPlayer _returnvalue_2)
  (Default|LocalSetPlayerName _returnvalue_2))

(event Custom|SpawnPlayer
  (params (PlayerController :type Player%20Controller%20Object%20Reference))
  (bind _returnvalue (Pawn|GetControlledPawn PlayerController))
  ;[1 0.7467 0.5294] Spawn a player
  (bind _asjump_controller (Utilities|Casting|CastToJUMP_Controller PlayerController))
  (if (Variables|/Game/Blueprints/JUMP_Controller.JUMP_Controller_C|GetIsLoaded? _asjump_controller) :!label _label
    (Utilities|IsValid _returnvalue
      (:Is%20Valid
        (Actor|DestroyActor _returnvalue))
      (:Is%20Not%20Valid
        _))
    (bind _returnvalue_2 (CallFunction|GetSpawnTransform _asjump_controller))
    (bind _returnvalue_3 (Game|SpawnActorfromClass "/Game/Blueprints/JUMP_Player.JUMP_Player_C" _returnvalue_2 "AdjustIfPossibleButAlwaysSpawn" _asjump_controller _asjump_controller 0))
    (Pawn|Possess _asjump_controller _returnvalue_3)
    (Default|SetLocalOwningPlayer _returnvalue_3)
    (Default|LocalSetPlayerName _returnvalue_3)
    (else
      (Default|Load _asjump_controller)
      (Utilities|FlowControl|RetriggerableDelay 0.5)
      (goto _label))))

(event Custom|Alert
  (params (Message :type Text) (Color :type Linear%20Color%20Structure))
  ;[1 1 1] Chat
  (for _array_element (Variables|Default|GetAllPlayerControllers)
    (bind _asjump_controller (Utilities|Casting|CastToJUMP_Controller _array_element))
    (Default|ReceiveAlert _asjump_controller Message Color)))

(event Custom|Set%20Spawn%20Points
  ;[1 1 1] Set spawn points
  (if (not (and (> (Utilities|Array|Length (Variables|Default|GetDefaultSpawnPoints)) 0) (> (Utilities|Array|Length (Variables|Default|GetTutorialSpawnPoints)) 0)))
    (bind _outactors (Actor|GetAllActorsOfClass "/Script/Engine.PlayerStart"))
    (Variables|Default|SetDefaultSpawnPoints _outactors)
    (Utilities|Array|Clear (Variables|Default|GetTutorialSpawnPoints))
    (bind _outactors_2 (Actor|GetAllActorsOfClass "/Game/Blueprints/Scene/RespawnPoint.RespawnPoint_C"))
    (for _array_element _outactors_2
      (if (Variables|/Game/Blueprints/Scene/RespawnPoint.RespawnPoint_C|GetisTutorial? _array_element)
        (Utilities|Array|Add (Variables|Default|GetTutorialSpawnPoints) _array_element)))))

(event Custom|CheckPlayerHighScores
  (params (player :type JUMP%20Controller%20Object%20Reference))
  (Default|LocalCheckHighscores player (Variables|Default|GetLevelManagers)))

(event EventBeginPlay)

(event EventPostLogin
  (params (NewPlayer :type Player%20Controller%20Object%20Reference))
  ;[0.4623 0.8065 1] New Player Joined
  (CallFunction|SetSpawnPoints)
  (Networking|SwitchHasAuthority
    (:Authority
      (Utilities|Array|Add (Variables|Default|GetAllPlayerControllers) NewPlayer)
      (if (== (Utilities|Array|Length (Variables|Default|GetLevelManagers)) 0)
        (CallFunction|GetLevelManagers))
      (bind _asjump_controller (Utilities|Casting|CastToJUMP_Controller NewPlayer))
      (Default|Load _asjump_controller)
      (CallFunction|SpawnPlayer NewPlayer))))

(event EventOnLogout
  (params (ExitingController :type Controller%20Object%20Reference))
  ;[0.4623 0.8065 1] Player Left
  (bind _asjump_controller (Utilities|Casting|CastToJUMP_Controller ExitingController))
  (Utilities|Array|RemoveItem (Variables|Default|GetAllPlayerControllers) _asjump_controller)
  (bind _asjump_controller_2 (Utilities|Casting|CastToJUMP_Controller ExitingController))
  (CallFunction|Alert (Utilities|Text|FormatText "{Name} has left the server." (Utilities|Text|ToText(String) (Class|AdvancedSessionsLibrary|GetPlayerName _asjump_controller_2))) "(R=0.000000,G=0.041267,B=0.895833,A=1.000000)"))

(fn ConstructionScript
  (bind _outactors (Actor|GetAllActorsOfClass 0)))

(fn GetSpawnTransform
  (params (Controller :type JUMP%20Controller%20Object%20Reference))
  (bind _defaultspawnpoints (Variables|Default|GetDefaultSpawnPoints))
  (bind _tutorialspawnpoints (Variables|Default|GetTutorialSpawnPoints))
  (if (Variables|/Game/Blueprints/JUMP_Controller.JUMP_Controller_C|GetCompletedTutorial? Controller)
    (return (Transformation|GetActorTransform (Utilities|Array|Get(acopy) _defaultspawnpoints (Math|Random|RandomIntegerinRange 0 (- (Utilities|Array|Length _defaultspawnpoints) 1)))))
    (else
      (return (Transformation|GetActorTransform (Utilities|Array|Get(acopy) _tutorialspawnpoints (Math|Random|RandomIntegerinRange 0 (- (Utilities|Array|Length _tutorialspawnpoints) 1))))))))