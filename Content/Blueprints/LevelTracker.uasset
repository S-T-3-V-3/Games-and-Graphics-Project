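; Tracks one player's run through a level: attempt count, elapsed time and the level UI.
; Start, end and reset events control a Tick-driven timer, with each start counting an attempt.
; Attempt totals and first and best completion times are saved per level index in JumpGameInstance, growing the score array as needed.
; Every completion also goes to the Controller's server high-score comparison under the player's Steam name.
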(event Custom|Initialize
  (params (LevelInfo :type Level%20Info%20Structure) (LevelManager :type Level%20Manager%20Object%20Reference))
  (Variables|Default|SetLevelInfo LevelInfo)
  (Variables|Default|SetTimeElapsed 0.0)
  (Variables|Default|SetLevelManager LevelManager)
  (CallFunction|AddLevelUI))

(event Custom|RemoveLevelUI
  (Widget|RemovefromParent (Variables|Default|GetActiveLevelUI)))

(event Custom|Reset
  (Utilities|FlowControl|Delay 0.1)
  (Variables|Default|SetTimeElapsed 0.0)
  (Variables|Default|SetisActive? false))

(event Custom|StartTimer
  (Variables|Default|SetisActive? true)
  (Math|Integer|IncrementInt (Variables|Default|GetNumAttempts)))

(event Custom|AddLevelUI
  (bind _returnvalue (UserInterface|CreateWidget "/Game/Blueprints/UI/LevelUI.LevelUI_C" (Game|GetPlayerController 0)))
  (bind _output_get (Variables|Default|SetActiveLevelUI _returnvalue))
  (UserInterface|Viewport|AddtoViewport _output_get 0))

(event Custom|EndTimer
  (Variables|Default|SetisActive? false))

(event Custom|OnLevelComplete
  (params (Manager :type Level%20Manager%20Object%20Reference))
  (bind _returnvalue (Math|DateTime|UTCNow))
  (bind _numattempts (Variables|Default|GetNumAttempts))
  (bind _timeelapsed (Variables|Default|GetTimeElapsed))
  (bind _levelresult (Utilities|Struct|MakeLevelResult _timeelapsed _returnvalue _numattempts))
  (bind _result (CallFunction|GetLevelScore (.levelindex (Variables|Default|GetLevelInfo))))
  (Utilities|FlowControl|Sequence
    (:then_0
      (if (.completed? _result)
        ;[1 1 1] Check if new record
        (if (< (Variables|Default|GetTimeElapsed) (.score (.bestresult _result)))
          ;[1 1 1] Set new best result
          (bind _asjump_game_instance (Utilities|Casting|CastToJumpGameInstance (Game|GetGameInstance)))
          (Utilities|Struct|SetmembersinPlayerLevelInfo (Utilities|Array|Get(acopy) (Variables|/Game/Blueprints/JumpGameInstance.JumpGameInstance_C|GetCurrentPlayerScores _asjump_game_instance) (.levelindex (Variables|Default|GetLevelInfo))) (Utilities|Struct|MakeLevelResult (Variables|Default|GetTimeElapsed) (Math|DateTime|UTCNow) (+ (.TotalAttempts (Utilities|Struct|BreakPlayerLevelInfo (Utilities|Array|Get(acopy) (Variables|/Game/Blueprints/JumpGameInstance.JumpGameInstance_C|GetCurrentPlayerScores _asjump_game_instance) (.levelindex (Variables|Default|GetLevelInfo))))) (Variables|Default|GetNumAttempts))))
          (Default|Save _asjump_game_instance))
        (else
          ;[1 1 1] Set Both First + Best Results
          (bind _asjump_game_instance_2 (Utilities|Casting|CastToJumpGameInstance (Game|GetGameInstance)))
          (Utilities|Array|SetArrayElem (Variables|/Game/Blueprints/JumpGameInstance.JumpGameInstance_C|GetCurrentPlayerScores _asjump_game_instance_2) (.levelindex (Variables|Default|GetLevelInfo)) (Utilities|Struct|MakePlayerLevelInfo true _levelresult _levelresult 0) true)
          (Default|Save _asjump_game_instance_2))))
    (:then_1
      (bind _returnvalue_2 (Class|AdvancedSteamFriendsLibrary|GetSteamPersonaName (Class|AdvancedSteamFriendsLibrary|GetLocalSteamIDfromSteam)))
      (Default|ServerCompareHighScore (Variables|Default|GetController) (Utilities|Struct|MakeLevelResult (Variables|Default|GetTimeElapsed) (Math|DateTime|UTCNow) (Variables|Default|GetNumAttempts)) (Utilities|Text|ToText(String) _returnvalue_2) Manager))))

(event Custom|UpdateStats
  (bind _levelinfo (Variables|Default|GetLevelInfo))
  (bind _asjump_game_instance (Utilities|Casting|CastToJumpGameInstance (Game|GetGameInstance)))
  (if (>= (.levelindex _levelinfo) (Utilities|Array|Length (Variables|/Game/Blueprints/JumpGameInstance.JumpGameInstance_C|GetCurrentPlayerScores _asjump_game_instance)))
    (Utilities|Array|SetArrayElem (Variables|/Game/Blueprints/JumpGameInstance.JumpGameInstance_C|GetCurrentPlayerScores _asjump_game_instance) (.levelindex _levelinfo) (Utilities|Struct|MakePlayerLevelInfo false "(Score_21_0CF7B57648313D4F8B7F268E6F6445F0=0.000000,ScoreDateTime_22_6654ECDA4637DE2B3980B289DD1FC8F6=0001.01.01-00.00.00,TotalAttempts_16_12F51F26434202628902ACB6E30B881D=0)" "(Score_21_0CF7B57648313D4F8B7F268E6F6445F0=0.000000,ScoreDateTime_22_6654ECDA4637DE2B3980B289DD1FC8F6=0001.01.01-00.00.00,TotalAttempts_16_12F51F26434202628902ACB6E30B881D=0)" (Variables|Default|GetNumAttempts)) true)
    (else
      (Utilities|Struct|SetmembersinPlayerLevelInfo (Utilities|Array|Get(acopy) (Variables|/Game/Blueprints/JumpGameInstance.JumpGameInstance_C|GetCurrentPlayerScores _asjump_game_instance) (.levelindex _levelinfo)) (+ (.TotalAttempts (Utilities|Struct|BreakPlayerLevelInfo (Utilities|Array|Get(acopy) (Variables|/Game/Blueprints/JumpGameInstance.JumpGameInstance_C|GetCurrentPlayerScores _asjump_game_instance) (.levelindex _levelinfo)))) (Variables|Default|GetNumAttempts)))))
  (Default|Save _asjump_game_instance))

(event EventBeginPlay)

(event EventTick
  (params (DeltaSeconds :type Float%20%28single-precision%29))
  (if (Variables|Default|GetisActive?)
    (Variables|Default|SetTimeElapsed (+ DeltaSeconds (Variables|Default|GetTimeElapsed)))))

(fn GetLevelScore
  (params (Level :type Integer))
  (bind _returnvalue (Game|GetGameInstance))
  (bind _asjump_game_instance (Utilities|Casting|CastToJumpGameInstance _returnvalue))
  (bind _currentplayerscores (Variables|/Game/Blueprints/JumpGameInstance.JumpGameInstance_C|GetCurrentPlayerScores _asjump_game_instance))
  (if (>= (Utilities|Array|Length _currentplayerscores) (+ Level 1))
    _
    (else
      (Utilities|Array|SetArrayElem _currentplayerscores Level (Utilities|Struct|MakePlayerLevelInfo false "(Score_21_0CF7B57648313D4F8B7F268E6F6445F0=0.000000,ScoreDateTime_22_6654ECDA4637DE2B3980B289DD1FC8F6=0001.01.01-00.00.00,TotalAttempts_16_12F51F26434202628902ACB6E30B881D=0)" "(Score_21_0CF7B57648313D4F8B7F268E6F6445F0=0.000000,ScoreDateTime_22_6654ECDA4637DE2B3980B289DD1FC8F6=0001.01.01-00.00.00,TotalAttempts_16_12F51F26434202628902ACB6E30B881D=0)" 0) true)))
  (return (Utilities|Array|Get(acopy) _currentplayerscores Level)))